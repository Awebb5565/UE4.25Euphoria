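; Weapon base actor that ALS characters pick up by walking into its box, then fire and reload.
; Overlap claims the character's empty primary or secondary slot, chosen by the Secondary flag, through its WeaponSystemComponent.
; Fire spends ammo, line-traces between caller-supplied points, sends character hits to BPEuphoriaComponent with an attached flesh decal, and plays muzzle flash, sound and animation.
; Reload instantly refills to MaxAmmo.
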(event OnComponentBeginOverlap(Box)
  (params (OverlappedComponent :type Primitive%20Component%20Object%20Reference) (OtherActor :type Actor%20Object%20Reference) (OtherComp :type Primitive%20Component%20Object%20Reference) (OtherBodyIndex :type Integer) (bFromSweep :type Boolean) (SweepResult :type Hit%20Result%20Structure%20%28by%20ref%29))
  (bind _self self)
  (bind _secondary_ (Variables|Default|GetSecondary?))
  ;[1 1 1] Adding Weapons
  (bind _asals_anim_man_character_bp (Utilities|Casting|CastToALS_AnimMan_CharacterBP OtherActor))
  (if _secondary_
    (Utilities|IsValid (Variables|/Game/WeaponSystem/WeaponSystemComponent.WeaponSystemComponent_C|GetSecondary%20Weapon (Variables|/Game/AdvancedLocomotionV4/Blueprints/CharacterLogic/ALS_AnimMan_CharacterBP.ALS_AnimMan_CharacterBP_C|GetWeaponSystemComponent _asals_anim_man_character_bp))
      (:Is%20Not%20Valid
        (if (not (Variables|Default|GetEquipped))
          (bind _output_get (Variables|/Game/WeaponSystem/WeaponSystemComponent.WeaponSystemComponent_C|SetSecondary%20Weapon (Variables|/Game/AdvancedLocomotionV4/Blueprints/CharacterLogic/ALS_AnimMan_CharacterBP.ALS_AnimMan_CharacterBP_C|GetWeaponSystemComponent _asals_anim_man_character_bp) _self))
          (Default|PickupWeapon (Variables|/Game/AdvancedLocomotionV4/Blueprints/CharacterLogic/ALS_AnimMan_CharacterBP.ALS_AnimMan_CharacterBP_C|GetWeaponSystemComponent _asals_anim_man_character_bp) _output_get _secondary_)
          (Variables|Default|SetEquipped true))))
    (else
      (Utilities|IsValid (Variables|/Game/WeaponSystem/WeaponSystemComponent.WeaponSystemComponent_C|GetPrimary%20Weapon (Variables|/Game/AdvancedLocomotionV4/Blueprints/CharacterLogic/ALS_AnimMan_CharacterBP.ALS_AnimMan_CharacterBP_C|GetWeaponSystemComponent _asals_anim_man_character_bp))
        (:Is%20Not%20Valid
          (if (not (Variables|Default|GetEquipped))
            (bind _output_get_2 (Variables|/Game/WeaponSystem/WeaponSystemComponent.WeaponSystemComponent_C|SetPrimary%20Weapon (Variables|/Game/AdvancedLocomotionV4/Blueprints/CharacterLogic/ALS_AnimMan_CharacterBP.ALS_AnimMan_CharacterBP_C|GetWeaponSystemComponent _asals_anim_man_character_bp) _self))
            (Default|PickupWeapon (Variables|/Game/AdvancedLocomotionV4/Blueprints/CharacterLogic/ALS_AnimMan_CharacterBP.ALS_AnimMan_CharacterBP_C|GetWeaponSystemComponent _asals_anim_man_character_bp) _output_get_2 _secondary_)
            (Variables|Default|SetEquipped true)))))))

(event EventBeginPlay)

(event Collision|EventActorBeginOverlap
  (params (OtherActor :type Actor%20Object%20Reference)))

(event EventTick
  (params (DeltaSeconds :type Float%20%28single-precision%29)))

(fn ConstructionScript)

(fn Fire
  (params (Start%20Line%20Trace :type Vector) (End%20Line%20Trace :type Vector))
  (bind _skeletalmesh (Variables|Default|GetSkeletalMesh))
  (bind _current_ammo (Variables|Default|GetCurrent%20Ammo))
  (bind _returnvalue (Transformation|GetSocketTransform _skeletalmesh "muzzleSocket" "RTS_World"))
  ;[1 1 1] Fire Logic
  (if (Variables|Default|GetEquipped)
    (if (not (<= _current_ammo 0))
      (Math|Integer|DecrementInt _current_ammo
        (:%20%20
          (Utilities|FlowControl|Sequence
            (:then_0
              (bind (_outhit _returnvalue_2) (Collision|LineTraceByChannel Start%20Line%20Trace End%20Line%20Trace "TraceTypeQuery1" false 0 "None"))
              (if _returnvalue_2
                (Utilities|FlowControl|Sequence
                  (:then_0
                    (bind _asals_anim_man_character_bp (Utilities|Casting|CastToALS_AnimMan_CharacterBP (.HitActor (Collision|BreakHitResult _outhit))))
                    (Default|HitFunction (Variables|/Game/AdvancedLocomotionV4/Blueprints/CharacterLogic/ALS_AnimMan_CharacterBP.ALS_AnimMan_CharacterBP_C|GetBP_EuphoriaComponent _asals_anim_man_character_bp) (.HitBoneName (Collision|BreakHitResult _outhit)) (Variables|Default|GetDamage) (+ (.ImpactPoint (Collision|BreakHitResult _outhit)) 1522.0) (.ImpactPoint (Collision|BreakHitResult _outhit)))
                    (bind _returnvalue_3 (Class|GameplayStatics|SpawnDecalAttached (Utilities|Select :Index (Math|Random|RandomIntegerinRange 0 3) :Option%200 "/Game/UWC_Bullet_Holes/Instances/Decals/Flesh/MI_Flesh_1.MI_Flesh_1" :Option%201 "/Game/UWC_Bullet_Holes/Instances/Decals/Flesh/MI_Flesh_2.MI_Flesh_2" :Option%202 "/Game/UWC_Bullet_Holes/Instances/Decals/Flesh/MI_Flesh_3.MI_Flesh_3") "-7.000000,-7.000000,-7.000000" (.HitComponent (Collision|BreakHitResult _outhit)) (.HitBoneName (Collision|BreakHitResult _outhit)) (.ImpactPoint (Collision|BreakHitResult _outhit)) (Math|Conversions|RotationFromXVector (.ImpactNormal (Collision|BreakHitResult _outhit))) "KeepWorldPosition" 0.0))
                    (Variables|/Game/EuphoriaComponent/EuphoriaComponent.EuphoriaComponent_C|SetLastWoundLocation (Variables|/Game/AdvancedLocomotionV4/Blueprints/CharacterLogic/ALS_AnimMan_CharacterBP.ALS_AnimMan_CharacterBP_C|GetBP_EuphoriaComponent _asals_anim_man_character_bp) _returnvalue_3)))))
            (:then_1
              (Effects|SpawnEmitterAttached (Variables|Default|GetMuzzle%20Flash) _skeletalmesh "muzzleSocket" (.location _returnvalue) (.rotation _returnvalue) "1.000000,1.000000,1.000000" "KeepWorldPosition")
              (Audio|SpawnSoundAttached (Variables|Default|GetGun%20Sounds) _skeletalmesh "None" "0, 0, 0" "0, 0, 0" "KeepRelativeOffset" false 1.0 1.0 0.0 0 0)
              (Components|Animation|PlayAnimation (Variables|Default|GetSkeletalMesh) (Variables|Default|GetWeapon%20Animation) false))))))))

(fn Reload
  ;[1 1 1] Reload Logic
  (if (not (>= (Variables|Default|GetCurrent%20Ammo) (Variables|Default|GetMax%20Ammo)))
    (Variables|Default|SetCurrent%20Ammo (Variables|Default|GetMax%20Ammo))))